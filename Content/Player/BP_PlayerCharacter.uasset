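; Player character Blueprint with single-axis movement along world X and jumping through Enhanced Input.
; Entering Falling movement mode sets a CoyoteTime flag, which a retriggerable delay clears after a short grace window.
; Pressing jump during that window also adds an upward LaunchCharacter impulse.
; The flag is set for any fall, including after a jump, and is not cleared on use, so repeated mid-air launches are possible.
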(event `EnhancedInput|/Game/Inputs/IA_Move`
  (params (ActionValue :type "Vector2D Structure") (ElapsedSeconds :type "Float (double-precision)") (TriggeredSeconds :type "Float (double-precision)") (InputAction :type "InputAction Object Reference" :default "/Game/Inputs/IA_Move.IA_Move"))
  ;[0.15 0.03036 0.1235 0.5] Character movement on X axis
  (:`Triggered`
    (`self.AddMovementInput` (1.0 0.0 0.0) ActionValue_X)))

(event `EnhancedInput|/Game/Inputs/IA_Jump`
  (params (ActionValue :type Boolean) (ElapsedSeconds :type "Float (double-precision)") (TriggeredSeconds :type "Float (double-precision)") (InputAction :type "InputAction Object Reference" :default "/Game/Inputs/IA_Jump.IA_Jump"))
  ;[0.15 0.04186 0.1237 0.5] When pressed activate jump,
  (:`Started`
    (`self.Jump`)
    ;[0.15 0.055 0.135 0.5] If in Coyote time allow midair jump
    (if (`self.Coyote Time`)
      (`self.LaunchCharacter` (0.0 0.0 600.0))))
  (:`Completed`
    (`self.StopJumping`)))

(event `self.K2_OnMovementModeChanged`
  (params (PrevMovementMode :type "EMovementMode Enum" :default "MOVE_None") (NewMovementMode :type "EMovementMode Enum" :default "MOVE_None") (PrevCustomMode :type Byte) (NewCustomMode :type Byte))
  ;[0.15 0.04556 0.1142 0.5] If player is falling, allow 0.4 seconds of coyote time to jump.
  (if (`|EnumEquality` NewMovementMode "MOVE_Falling")
    (set `self.Coyote Time` true)
    (`KismetSystemLibrary.RetriggerableDelay` 0.4)
    (set `self.Coyote Time` false)))

(fn `UserConstructionScript`)