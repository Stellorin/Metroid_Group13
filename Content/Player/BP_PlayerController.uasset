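; Player controller Blueprint that sets up the player's input on game start.
; BeginPlay adds the IMC_PlayerControls mapping context to the Enhanced Input local player subsystem at priority zero.
; The horizontal axis and Tick events are empty, and leftover movement code that offsets the pawn along a normalized direction is disconnected and marked as unused.
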(event `self.ReceiveBeginPlay`
  ;[0.15 0.04301 0.1398 0.5] In use mapping context
  (`EnhancedInputSubsystemInterface.AddMappingContext` (subsystem `EnhancedInputLocalPlayerSubsystem`) "/Game/Inputs/IMC_PlayerControls.IMC_PlayerControls" 0 (struct)))

(event `InputAxis|Horizontal Input`
  (params (AxisValue :type "Float (single-precision)"))
  ; Old Code NOT BEING USED CURRENTLY
  ;; Map horizontal inputs
)

(event `self.ReceiveTick`
  (params (DeltaSeconds :type "Float (single-precision)"))
  ; Old Code NOT BEING USED CURRENTLY
  ;; Get the player to actually move
)

(fn `UserConstructionScript`)